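; Player controller for SpecSpace3D that sets up input and camera view and relays movement and jump input.
; On possess it adds the IMC_Test Enhanced Input mapping context to the first local player.
; At BeginPlay it blends the view target to the BP_SpecSpaceCameraRig found in the level.
; Move and jump actions pass their values straight to OnMoveAxis and OnJump, with no movement logic in the controller.
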(event `self.ReceivePossess`
  (params (PossessedPawn :type "Pawn Object Reference"))
  (`EnhancedInputSubsystemInterface.AddMappingContext` (pcsubsystem `EnhancedInputLocalPlayerSubsystem` (`GameplayStatics.GetPlayerController` 0)) "/Game/Input/IMC_Test.IMC_Test" 0 (struct)))

(event `self.ReceiveBeginPlay`
  (bind _returnvalue (`GameplayStatics.GetActorOfClass` "/Game/SpecSpace3D/UniqueObjects/BP_SpecSpaceCameraRig.BP_SpecSpaceCameraRig_C"))
  (`self.SetViewTargetWithBlend` (`GameplayStatics.GetPlayerController` 0) _returnvalue 0.3 "VTBlend_Linear" 0.0 false))

(event `EnhancedInput|/Game/Input/IA_Move`
  (params (ActionValue :type "Vector2D Structure") (ElapsedSeconds :type "Float (double-precision)") (TriggeredSeconds :type "Float (double-precision)") (InputAction :type "InputAction Object Reference" :default "/Game/Input/IA_Move.IA_Move"))
  (:`Triggered`
    (`self.OnMoveAxis` ActionValue)))

(event `EnhancedInput|/Game/Input/IA_Jump`
  (params (ActionValue :type Boolean) (ElapsedSeconds :type "Float (double-precision)") (TriggeredSeconds :type "Float (double-precision)") (InputAction :type "InputAction Object Reference" :default "/Game/Input/IA_Jump.IA_Jump"))
  (:`Triggered`
    (`self.OnJump` ActionValue)))

(fn `UserConstructionScript`)